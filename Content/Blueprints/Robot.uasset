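; Robot Blueprint that walks to an interacted room item or door and performs its interaction.
; MovetoTarget uses AI MoveTo to reach the item's interact point or the door's inside point, then a timeline lerps rotation to face it.
; Items then run MyInteraction; open doors get a second move offset along their facing.
; Success or failure, the robot then teleports to the outside point and activates the next room.
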(event `self.MoveToTarget`
  (params (InteractedItem_Instigator :type "HInteractedItem Object Reference"))
  (bind _interacted_item_instigator (`self.Interacted Item Instigator`))
  ;[1 1 1] 机器人寻路到目标点
  (bind _output_get (set `self.Interacted Item Instigator` InteractedItem_Instigator))
  (bind _ashitem_in_room (cast `HItemInRoom` _output_get)
    (:`then`
      (bind _returnvalue (`HItemInRoom.GetInteractPointLocation` _ashitem_in_room))
      (bind _returnvalue_2 (`HItemInRoom.GetInteractPointRotator` _ashitem_in_room))
      (set `self.TargetRotation` _returnvalue_2)
      (`AITask_MoveTo.AIMoveTo` (`AIBlueprintHelperLibrary.GetAIController` self) _returnvalue null 2.0
        (:`then`
          (`KismetSystemLibrary.PrintString` "开始移动"))
        (:`OnRequestFailed`
          (`KismetSystemLibrary.PrintString` "移动失败" true true (struct :`R` 1.0 :`G` 1.0 :`A` 1.0) 10.0))
        (:`OnMoveFinished`
          (`KismetSystemLibrary.PrintString` "移动完成")
          ;[1 1 1] 机器人移动到目标点之后修正朝向
          (set `self.MyRotation` (`self.K2_GetActorRotation`) :!label _label)
          (bind (_direction _alpha) (`Timeline|TurnToTargetDoor` :!via `PlayFromStart`)
            (:`Update`
              (`self.K2_SetActorRotation` (`KismetMathLibrary.RLerp` (`self.MyRotation`) (`self.TargetRotation`) _alpha)))
            (:`Finished`
              (bind _ashitem_in_room_2 (cast `HItemInRoom` _interacted_item_instigator)
                (:`then`
                  (`HItemInRoom.MyInteraction` _ashitem_in_room_2 null)
                  (`KismetSystemLibrary.PrintString` "机器人触发了房间内可交互物品的逻辑" true false))
                (:`CastFailed`
                  (bind _ashdoor (cast `HDoor` _interacted_item_instigator))
                  (bind _returnvalue_3 (`HDoor.GetDoorIsClosed` _ashdoor))
                  (if _returnvalue_3
                    (`KismetSystemLibrary.PrintString` "门是关闭的" true true (struct :`G` 1.0 :`B` 1.0 :`A` 1.0))
                    (else
                      (bind _returnvalue_4 (`HDoor.GetInDoorLoaction` _ashdoor))
                      (bind _returnvalue_5 (`HDoor.GetInDoorRotatior` _ashdoor))
                      (`AITask_MoveTo.AIMoveTo` (`AIBlueprintHelperLibrary.GetAIController` self) (+ _returnvalue_4 (* (`KismetMathLibrary.GetForwardVector` _returnvalue_5) (`self.OutDoorDistance`))) null
                        (:`then`
                          (`KismetSystemLibrary.PrintString` "准备出门"))
                        (:`OnRequestFailed`
                          (`KismetSystemLibrary.PrintString` "出门失败")
                          (bind _returnvalue_6 (`HDoor.GetOutDoorLoaction` _ashdoor :!label _label_2))
                          (bind _returnvalue_7 (`HDoor.GetOutDoorRotatior` _ashdoor))
                          (`self.K2_SetActorLocationAndRotation` _returnvalue_6 _returnvalue_7)
                          (`HDoor.ActiveNextRoom` _ashdoor))
                        (:`OnMoveFinished`
                          (`KismetSystemLibrary.PrintString` "出门成功")
                          (goto _label_2))))))))))))
    (:`CastFailed`
      (bind _ashdoor_2 (cast `HDoor` _output_get))
      (bind _returnvalue_8 (`HDoor.GetInDoorLoaction` _ashdoor_2))
      (bind _returnvalue_9 (`HDoor.GetInDoorRotatior` _ashdoor_2))
      (set `self.TargetRotation` _returnvalue_9)
      (`AITask_MoveTo.AIMoveTo` (`AIBlueprintHelperLibrary.GetAIController` self) _returnvalue_8 null 2.0
        (:`then`
          (`KismetSystemLibrary.PrintString` "开始移动"))
        (:`OnRequestFailed`
          (`KismetSystemLibrary.PrintString` "移动失败" true true (struct :`R` 1.0 :`G` 1.0 :`A` 1.0) 10.0))
        (:`OnMoveFinished`
          (`KismetSystemLibrary.PrintString` "移动完成")
          (goto _label))))))

(fn `UserConstructionScript`)