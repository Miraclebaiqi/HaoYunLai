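; Interactable in-game monitor that shows live views of Room actors and lets the player jump into the displayed room's camera.
; BeginPlay gathers all Rooms and points one's SceneCapture2D at a shared render target.
; Interact stores the player; FurtherInteraction switches their camera to that room and sets the room-focus state.
; Left/right arrows cycle a wrapped index, either moving the render target or switching the player's camera, depending on player state.
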(event `self.ReceiveBeginPlay`
  (bind _outactors (`GameplayStatics.GetAllActorsOfClass` "/Game/Blueprints/Room.Room_C"))
  (bind _output_get (set `self.Rooms` _outactors))
  (bind _output (`|GetArrayItem` _output_get (`self.RoomIndex`)))
  (`/Engine/EditorBlueprintResources/StandardMacros.IsValid` _output
    (:`Is Valid`
      (set `SceneCaptureComponent2D.TextureTarget` "/Game/Materials/RT_Monitor.RT_Monitor" (`self.GetComponentByClass` _output "/Script/Engine.SceneCaptureComponent2D"))
      (set `self.CurrentCamera` _output))
    (:`Is Not Valid`
      (`KismetSystemLibrary.PrintString` "监视器获取摄像机异常" true true (struct :`R` 1.0 :`G` 0.5 :`A` 1.0) 10.0))))

(event `HGameInterface.Interact`
  (params (InstigatorActor :type "Pawn Object Reference"))
  (`parent.Interact` InstigatorActor)
  (bind _asplayer (cast `/Game/Blueprints/Player` InstigatorActor)
    (:`then`
      (set `self.As Player` _asplayer)
      (`KismetSystemLibrary.PrintString` "监视器交互，设定玩家"))
    (:`CastFailed`
      (`KismetSystemLibrary.PrintString` "监视器交互触发者异常" true true (struct :`R` 1.0 :`G` 0.5 :`A` 1.0) 10.0))))

(event `self.FurtherInteraction`
  (params (InstigatorActor :type "Pawn Object Reference"))
  (bind _currentcamera (`self.CurrentCamera`))
  (`KismetSystemLibrary.PrintString` "进入监视器深层逻辑")
  (bind _asplayer (cast `/Game/Blueprints/Player` InstigatorActor)
    (:`then`
      (`HPlayer.SwitchCurrentCamera` _asplayer _currentcamera)
      (`HRoomBase.RoomFocusOn` _currentcamera)
      (`HPlayer.SetPlayerState` _asplayer "PS_FocusInRoom")
      (set `self.IsFocused` false))
    (:`CastFailed`
      (`KismetSystemLibrary.PrintString` "监视器深层逻辑触发者异常" true true (struct :`R` 1.0 :`G` 0.5 :`A` 1.0) 10.0))))

(event `InputAction|ArrowLeft`
  (params (Key :type "Key Structure"))
  ;[1 1 1] 聚焦到监视器之后的操作，以及切换房间
  (:`Pressed`
    (`KismetSystemLibrary.PrintString` "←")
    (switch `EPlayerState` (`HPlayer.PS` (`self.As Player`))
      (:`PS_FocusOnTableItem`
        (bind _result (`/Engine/EditorBlueprintResources/StandardMacros.DecrementInt` (`self.RoomIndex`))
          (:`  `
            (bind _index (`self.RoomIndex_Calculate` _result))
            (bind _output_get (set `self.RoomIndex` _index))
            (`self.MonitorScreenChange` _output_get))))
      (:`PS_FocusInRoom`
        (bind _result_2 (`/Engine/EditorBlueprintResources/StandardMacros.DecrementInt` (`self.RoomIndex`))
          (:`  `
            (bind _index_2 (`self.RoomIndex_Calculate` _result_2))
            (bind _output_get_2 (set `self.RoomIndex` _index_2))
            (`self.RoomChange` _output_get_2)))))))

(event `InputAction|ArrowRight`
  (params (Key :type "Key Structure"))
  ;[1 1 1] 聚焦到监视器之后的操作，以及切换房间
  (:`Pressed`
    (`KismetSystemLibrary.PrintString` "→")
    (switch `EPlayerState` (`HPlayer.PS` (`self.As Player`))
      (:`PS_FocusOnTableItem`
        (bind _result (`/Engine/EditorBlueprintResources/StandardMacros.IncrementInt` (`self.RoomIndex`))
          (:`  `
            (bind _index (`self.RoomIndex_Calculate` _result))
            (bind _output_get (set `self.RoomIndex` _index))
            (`self.MonitorScreenChange` _output_get))))
      (:`PS_FocusInRoom`
        (bind _result_2 (`/Engine/EditorBlueprintResources/StandardMacros.IncrementInt` (`self.RoomIndex`))
          (:`  `
            (bind _index_2 (`self.RoomIndex_Calculate` _result_2))
            (bind _output_get_2 (set `self.RoomIndex` _index_2))
            (`self.RoomChange` _output_get_2)))))))

(fn `MonitorScreenChange`
  (params (NewIndex :type Integer))
  (bind _output (`|GetArrayItem` (`self.Rooms`) NewIndex))
  (set `SceneCaptureComponent2D.TextureTarget` null (`self.GetComponentByClass` (`self.CurrentCamera`) "/Script/Engine.SceneCaptureComponent2D"))
  (set `SceneCaptureComponent2D.TextureTarget` "/Game/Materials/RT_Monitor.RT_Monitor" (`self.GetComponentByClass` _output "/Script/Engine.SceneCaptureComponent2D"))
  (set `self.CurrentCamera` _output))

(fn `RoomChange`
  (params (NewIndex :type Integer))
  (`HPlayer.SwitchCurrentCamera` (`self.As Player`) (`|GetArrayItem` (`self.Rooms`) NewIndex)))

(fn `RoomIndex_Calculate`
  (params (PerIndex :type Integer))
  (returns (Index :type Integer))
  (bind _returnvalue (`KismetArrayLibrary.Array_Length` (`self.Rooms`)))
  (bind _returnvalue_2 (mod PerIndex _returnvalue))
  (if (< _returnvalue_2 0)
    (return (+ _returnvalue_2 _returnvalue))
    (else
      (return _returnvalue_2))))

(fn `UserConstructionScript`
  (`parent.UserConstructionScript`))